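; BP_Bicycle is a player-controllable two-wheeled vehicle Blueprint built on a SimpleWheeledVehicleMovement component.
; Input axes map straight to per-wheel calls: MoveRight steers wheel 0, while MoveForward applies drive torque to wheel 1.
; The Handbreak action applies brake torque to wheel 1 while held and clears it on release.
; It uses no Tick or custom construction logic, and wheel indices are hardcoded.
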(event `InputAxis|MoveRight`
  (params (AxisValue :type "Float (single-precision)"))
  ;[1 1 1] Steering //Add more wheels if ne.
  (`SimpleWheeledVehicleMovementComponent.SetSteerAngle` (`self.SimpleWheeledVehicleMovement`) (* AxisValue 45.0) 0))

(event `InputAxis|MoveForward`
  (params (AxisValue :type "Float (single-precision)"))
  ;[1 1 1] Throttle
  (`SimpleWheeledVehicleMovementComponent.SetDriveTorque` (`self.SimpleWheeledVehicleMovement`) (* AxisValue 300.0) 1))

(event `InputAction|Handbreak`
  (params (Key :type "Key Structure"))
  (bind _simplewheeledvehiclemovement (`self.SimpleWheeledVehicleMovement`))
  ;[1 1 1] Handbreak
  (:`Pressed`
    (`SimpleWheeledVehicleMovementComponent.SetBrakeTorque` _simplewheeledvehiclemovement 3000.0 1))
  (:`Released`
    (`SimpleWheeledVehicleMovementComponent.SetBrakeTorque` _simplewheeledvehiclemovement 0.0 1)))

(fn `UserConstructionScript`
  (`parent.UserConstructionScript`))